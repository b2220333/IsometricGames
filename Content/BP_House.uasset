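; House Blueprint for a top-down game whose appearance follows its research level.
; The construction script adds one instance to the Base instanced mesh, then a macro switches on ResearchLevel to swap its mesh (cube, middle or roof) and set matching tier flags.
; BeginPlay caches the TopDownController reference, which is not used further here.
; The FloorCheck macro is an unfinished stub that nothing shown calls.
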(event EventBeginPlay
  (bind _astop_down_controller (Utilities|Casting|CastToTopDownController (Game|GetPlayerController 0)))
  (Variables|Default|SetPlayerControllerRef _astop_down_controller))

(fn ConstructionScript
  (Utilities|FlowControl|Sequence
    (:then_0
      ;[1 1 1] Base Generation
      (Components|InstancedStaticMesh|AddInstance (Variables|Default|GetBase) (Math|Transform|MakeTransform "0, 0, 0" "0, 0, 0" "1,1,1")))
    (:then_1
      (Utilities|ResearchMacro))))